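; BP_EXAMPLE_actor_with_lights_components is an example actor that reports how many point, spot and rect light components it has.
; Three separate custom events each gather one light type with GetComponentsByClass and print the count to screen as a debug string.
; Nothing in the graph calls these events; BeginPlay, overlap, Tick and the construction script are empty, and a leftover point light loop is never executed.
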(event Custom|count%20spots
  (Development|PrintString (Utilities|String|ToString(Integer) (Utilities|Array|Length (Actor|GetComponentsByClass "/Script/Engine.SpotLightComponent")))))

(event Custom|count_points
  (Development|PrintString (Utilities|String|ToString(Integer) (Utilities|Array|Length (Actor|GetComponentsByClass "/Script/Engine.PointLightComponent")))))

(event Custom|cout%20rect
  (Development|PrintString (Utilities|String|ToString(Integer) (Utilities|Array|Length (Actor|GetComponentsByClass "/Script/Engine.RectLightComponent")))))

(event EventBeginPlay)

(event Collision|EventActorBeginOverlap
  (params (OtherActor :type Actor%20Object%20Reference)))

(event EventTick
  (params (DeltaSeconds :type Float%20%28single-precision%29)))

(fn ConstructionScript)