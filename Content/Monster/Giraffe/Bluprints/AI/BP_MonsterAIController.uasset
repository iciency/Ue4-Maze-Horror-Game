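; BP_MonsterAIController is the AI controller for the Giraffe monster, running BT_MonsterAI on BeginPlay.
; Perception updates pass each updated actor to CheckPlayerActor, which writes the PlayerActorKey blackboard entry.
; That function works as a toggle: it clears the key if already valid, otherwise stores the sensed actor.
; It checks neither whether the actor is the player nor whether it was sensed or lost.
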(event OnPerceptionUpdated(AIPerception)
  (params (UpdatedActors :type Array%20of%20Actor%20Object%20References))
  (for _array_element UpdatedActors
    (CallFunction|CheckPlayerActor _array_element)))

(event EventBeginPlay
  (AI|RunBehaviorTree "/Game/Monster/Giraffe/Bluprints/AI/BT_MonsterAI.BT_MonsterAI"))

(fn ConstructionScript)

(fn CheckPlayerActor
  (params (SensedActor :type Actor%20Object%20Reference))
  (Utilities|IsValid (AI|Components|Blackboard|GetValueasObject (AI|GetBlackboard 0) (Utilities|Name|MakeLiteralName "PlayerActorKey"))
    (:Is%20Valid
      (AI|Components|Blackboard|SetValueasObject (AI|GetBlackboard 0) (Utilities|Name|MakeLiteralName "PlayerActorKey") 0))
    (:Is%20Not%20Valid
      (AI|Components|Blackboard|SetValueasObject (AI|GetBlackboard 0) (Utilities|Name|MakeLiteralName "PlayerActorKey") SensedActor))))