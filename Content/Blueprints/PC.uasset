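; Player controller that manages the in-game settings menu and quits the game on Escape.
; On BeginPlay outside IntroMap, it creates the BP_Setting widget, hides its exit panel, applies default and initial settings, and enables toggling.
; O calls OpenSetting, which adds the widget to the viewport once, then toggles its visibility, pause state, cursor and UI-only or game-only input.
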(event Custom|OpenSetting
  (bind _returnvalue (Game|GetPlayerController 0))
  (bind _bp_setting (Variables|Default|GetBP_Setting))
  (if (Variables|Default|GetIsLevel)
    (if (Variables|Default|GetIsSettingViewPort)
      (Widget|SetVisibility _bp_setting "Hidden")
      (Input|SetInputModeGameOnly _returnvalue)
      (Variables|Default|SetbShowMouseCursor false)
      (Game|SetGamePaused false)
      (Variables|Default|SetIsSettingViewPort false)
      (else
        (Utilities|FlowControl|Sequence
          (:then_0
            (Utilities|FlowControl|DoOnce false
              (:Completed
                (UserInterface|Viewport|AddtoViewport _bp_setting 0))))
          (:then_1
            (Widget|SetVisibility _bp_setting "SelfHitTestInvisible")
            (Input|SetInputModeUIOnly _returnvalue _bp_setting "DoNotLock")
            (Variables|Default|SetbShowMouseCursor true)
            (Game|SetGamePaused true)
            (Variables|Default|SetIsSettingViewPort true)))))))

(event EventBeginPlay
  (bind _returnvalue (Game|GetCurrentLevelName true))
  (if (Utilities|Enum|Equal(Enum) _returnvalue "IntroMap")
    (Variables|Default|SetIsLevel false)
    (else
      (Utilities|FlowControl|Sequence
        (:then_0
          (bind _returnvalue_2 (UserInterface|CreateWidget "/Game/Resource/UI/Intro/BP_Setting.BP_Setting_C" (Game|GetPlayerController 0)))
          (Variables|Default|SetBP_Setting _returnvalue_2)
          (Widget|SetVisibility (Variables|/Game/Resource/UI/Intro/BP_Setting.BP_Setting_C|GetExitPanel _returnvalue_2) "Hidden"))
        (:then_1
          (Default|DefualtSetting _returnvalue_2)
          (Default|InitSetting _returnvalue_2))
        (:then_2
          (Variables|Default|SetIsLevel true))))))

(event Input|KeyboardEvents|Escape
  (params (Key :type Key%20Structure :default "None"))
  (:Pressed
    (Game|QuitGame 0 "Quit" false)))

(event Input|KeyboardEvents|O
  (params (Key :type Key%20Structure :default "None"))
  (:Pressed
    (CallFunction|OpenSetting)))

(fn ConstructionScript)