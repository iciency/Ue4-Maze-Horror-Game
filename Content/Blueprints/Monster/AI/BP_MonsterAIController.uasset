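; BP_MonsterAIController is the monster's AI controller, which runs the BT_MonsterAI behavior tree on BeginPlay.
; AI perception updates pass each sensed actor to CheckPlayerActor, which writes it to the PlayerActorKey blackboard key only while that key holds no valid object.
; It does not verify that the actor is a player.
; Target perception info updates simply flip the IsPerception flag.
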(event OnPerceptionUpdated(AIPerception)
  (params (UpdatedActors :type Array%20of%20Actor%20Object%20References))
  (for _array_element UpdatedActors
    (CallFunction|CheckPlayerActor _array_element)))

(event OnTargetPerceptionInfoUpdated(AIPerception)
  (params (UpdateInfo :type Actor%20Perception%20Update%20Info%20Structure%20%28by%20ref%29))
  (bind _output_get (Variables|Default|SetIsPerception (not (stale _output_get)))))

(event EventBeginPlay
  (AI|RunBehaviorTree "/Game/Blueprints/Monster/AI/BT_MonsterAI.BT_MonsterAI"))

(fn ConstructionScript)

(fn CheckPlayerActor
  (params (SensedActor :type Actor%20Object%20Reference))
  (bind _returnvalue (AI|GetBlackboard 0))
  (bind _returnvalue_2 (Utilities|Name|MakeLiteralName "PlayerActorKey"))
  (Utilities|IsValid (AI|Components|Blackboard|GetValueasObject _returnvalue _returnvalue_2)
    (:Is%20Not%20Valid
      (AI|Components|Blackboard|SetValueasObject _returnvalue _returnvalue_2 SensedActor))))