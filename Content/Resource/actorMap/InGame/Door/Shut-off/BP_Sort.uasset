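; BP_Sort is a registry that orders the level's lever buttons, shut-off actors and modifier areas into index-addressable arrays.
; On BeginPlay it gathers all Button, Shutoff_2 and Modifierarea actors and sizes the Lever, Shutoff and Modifierarea arrays to match.
; Each actor replaces the slot given by its own number, Shutoffnum for buttons and Areanum for the others, so array index equals that ID.
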(event Custom|areaevent
  (bind _modifierarea (Variables|Default|Getmodifierarea))
  (bind _outactors (Actor|GetAllActorsOfClass "/Game/Resource/actorMap/InGame/Door/modifierarea/Modifierarea.Modifierarea_C"))
  (Utilities|Array|Resize _modifierarea (Utilities|Array|Length _outactors))
  (for _array_element _outactors
    (Utilities|Array|RemoveIndex _modifierarea (Variables|/Game/Resource/actorMap/InGame/Door/modifierarea/Modifierarea.Modifierarea_C|Getareanum _array_element))
    (Utilities|Array|Insert _modifierarea _array_element (Variables|/Game/Resource/actorMap/InGame/Door/modifierarea/Modifierarea.Modifierarea_C|Getareanum _array_element))))

(event Custom|eventshutoff
  (bind _shutoff (Variables|Default|Getshutoff))
  (bind _outactors (Actor|GetAllActorsOfClass "/Game/Resource/actorMap/InGame/Door/Shut-off/shut-off_2.shut-off_2_C"))
  (Utilities|Array|Resize _shutoff (Utilities|Array|Length _outactors))
  (for _array_element _outactors
    (Utilities|Array|RemoveIndex _shutoff (Variables|/Game/Resource/actorMap/InGame/Door/Shut-off/shut-off_2.shut-off_2_C|Getareanum _array_element))
    (Utilities|Array|Insert _shutoff _array_element (Variables|/Game/Resource/actorMap/InGame/Door/Shut-off/shut-off_2.shut-off_2_C|Getareanum _array_element))))

(event Custom|leverEvent
  (bind _lever (Variables|Default|Getlever))
  (bind _outactors (Actor|GetAllActorsOfClass "/Game/Resource/actorMap/InGame/Door/Shut-off/button.button_C"))
  (Utilities|Array|Resize _lever (Utilities|Array|Length _outactors))
  (for _array_element _outactors
    (Utilities|Array|RemoveIndex _lever (Variables|/Game/Resource/actorMap/InGame/Door/Shut-off/button.button_C|Getshutoffnum _array_element))
    (Utilities|Array|Insert _lever _array_element (Variables|/Game/Resource/actorMap/InGame/Door/Shut-off/button.button_C|Getshutoffnum _array_element))))

(event EventBeginPlay
  (CallFunction|LeverEvent)
  (CallFunction|Eventshutoff)
  (CallFunction|Areaevent))

(fn ConstructionScript)