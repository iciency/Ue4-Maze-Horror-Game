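; BP_Giraff is a monster that triggers a jumpscare when its capsule hits the first-person character.
; On BeginPlay it creates the BP_JumpSquare widget and computes a navigation path to the player, which it only prints, with no movement logic.
; A one-time guard on the hit plays a scare sound, shows the widget, then opens FirstPersonExampleMap after a short delay.
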(event OnComponentHit(CapsuleComponent)
  (params (HitComponent :type Primitive%20Component%20Object%20Reference) (OtherActor :type Actor%20Object%20Reference) (OtherComp :type Primitive%20Component%20Object%20Reference) (NormalImpulse :type Vector :default "0, 0, 0") (Hit :type Hit%20Result%20Structure%20%28by%20ref%29))
  (bind _returnvalue (Actor|GetActorOfClass "/Game/FirstPersonCPP/Blueprints/FirstPersonCharacter.FirstPersonCharacter_C"))
  (bind _output_get (Variables|Default|Setfirstpersoncharactor _returnvalue))
  (if (== OtherActor _output_get)
    (if (not (Variables|Default|Getonce))
      (Variables|Default|Setonce true)
      (Audio|PlaySound2D "/Game/Resource/Audio/InGame/Monster/catch/huggy-wuggy-jumscare_Cue.huggy-wuggy-jumscare_Cue" 1.0 1.0 0.0 0 0)
      (UserInterface|Viewport|AddtoViewport (Variables|Default|Getjumpscaure) 0)
      (Utilities|FlowControl|Delay 5.0)
      (Game|OpenLevel(byName) "FirstPersonExampleMap"))))

(event EventBeginPlay
  (bind _returnvalue (UserInterface|CreateWidget "/Game/Resource/UI/Jumpsquare/BP_JumpSquare.BP_JumpSquare_C"))
  (Variables|Default|Setjumpscaure _returnvalue)
  (bind _returnvalue_2 (Class|NavigationSystemV1|FindPathtoActorSynchronously (Transformation|GetActorLocation) (Game|GetPlayerCharacter 0) 1e+02 (AI|GetAIController self) "/Script/AIModule.NavFilter_AIControllerDefault"))
  (Development|PrintString (Utilities|GetDisplayName _returnvalue_2)))

(fn ConstructionScript)