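; BP_Monster is an enemy that turns toward the player and ends the encounter on contact.
; On BeginPlay it caches the first-person character and the BP_MonsterAIController found in the level.
; Each tick, while that controller's IsPerception flag is set, it rotates to face the player camera.
; A capsule hit with the player opens the "jumpSquhere" level, guarded by a DoOnce.
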(event OnComponentHit(CapsuleComponent)
  (params (HitComponent :type Primitive%20Component%20Object%20Reference) (OtherActor :type Actor%20Object%20Reference) (OtherComp :type Primitive%20Component%20Object%20Reference) (NormalImpulse :type Vector :default "0, 0, 0") (Hit :type Hit%20Result%20Structure%20%28by%20ref%29))
  (if (== OtherActor (Game|GetPlayerCharacter 0))
    (Utilities|FlowControl|DoOnce false
      (:Completed
        (Game|OpenLevel(byName) "jumpSquhere")))))

(event EventTick
  (params (DeltaSeconds :type Float%20%28single-precision%29))
  (bind _as_bp_monster_aicontroller (Variables|Default|GetAs%20BP%20Monster%20AIController))
  (Utilities|IsValid _as_bp_monster_aicontroller
    (:Is%20Valid
      (if (Variables|/Game/Resource/Monster/Bluprints/AI/BP_MonsterAIController.BP_MonsterAIController_C|GetIsPerception _as_bp_monster_aicontroller)
        (Transformation|SetActorRotation (Math|Rotator|FindLookatRotation (Transformation|GetActorLocation) (Transformation|GetActorLocation (Game|GetPlayerCameraManager 0))))))))

(event EventBeginPlay
  (bind _returnvalue (Actor|GetActorOfClass "/Game/Blueprints/FirstPersonCharacter.FirstPersonCharacter_C"))
  (Variables|Default|Setfirstpersoncharactor _returnvalue)
  (bind _returnvalue_2 (Actor|GetActorOfClass "/Game/Resource/Monster/Bluprints/AI/BP_MonsterAIController.BP_MonsterAIController_C"))
  (Variables|Default|SetAs%20BP%20Monster%20AIController _returnvalue_2))

(fn ConstructionScript)